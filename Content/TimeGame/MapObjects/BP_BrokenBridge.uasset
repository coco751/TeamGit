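; BP_BrokenBridge is a map object that breaks a bridge apart at game start and reassembles it on demand.
; On BeginPlay it gathers all BP_BridgeCube actors tagged "Movable", offsets each randomly along X and downward in Z, and clears IsPlaced.
; StartMoveToInitial plays a timeline that lerps each cube from its current transform toward its stored InitialLoc, setting IsPlaced on every update.
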(event Custom|Start%20Move%20To%20Initial
  (bind _assemble_bridge (Timeline|タイムライン Play)
    (:Update
      (for _array_element (Variables|Default|GetBridgeCube)
        (bind _asbp_bridge_cube (Utilities|Casting|CastToBP_BridgeCube _array_element))
        (Transformation|SetActorTransform _asbp_bridge_cube (Math|Transform|Lerp(Transform) (Transformation|GetActorTransform _asbp_bridge_cube) (Variables|/Game/TimeGame/MapObjects/BP_BridgeCube.BP_BridgeCube_C|GetInitialLoc _asbp_bridge_cube) _assemble_bridge))
        (Variables|/Game/TimeGame/MapObjects/BP_BridgeCube.BP_BridgeCube_C|SetIsPlaced _asbp_bridge_cube true)))))

(event EventBeginPlay
  (bind _outactors (Actor|GetAllActorsOfClasswithTag "/Game/TimeGame/MapObjects/BP_BridgeCube.BP_BridgeCube_C" "Movable"))
  (bind _output_get (Variables|Default|SetBridgeCube _outactors))
  (for _array_element _output_get
    (Transformation|SetActorTransform _array_element (Math|Transform|MakeTransform (+ (.location (Transformation|GetActorTransform _array_element)) (Math|Vector|MakeVector (Math|Random|RandomFloatinRange -5e+02 5e+02) 0.0 (Math|Random|RandomFloatinRange -5e+02 -2e+02))) "0, 0, 0" "1.000000,1.000000,1.000000"))
    (bind _asbp_bridge_cube (Utilities|Casting|CastToBP_BridgeCube _array_element))
    (Variables|/Game/TimeGame/MapObjects/BP_BridgeCube.BP_BridgeCube_C|SetIsPlaced _asbp_bridge_cube false)))

(fn ConstructionScript)